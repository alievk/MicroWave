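; Player controller that aims the controlled Burglar pawn toward the mouse cursor.
; Every tick it traces under the cursor on the Visibility channel and draws a debug arrow from the pawn to the hit location.
; It then casts the pawn to Burglar and sets its Yaw variable from the direction toward that point.
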(event `self.ReceiveTick`
  (params (DeltaSeconds :type "Float (single-precision)"))
  (bind _returnvalue (`self.K2_GetActorLocation` (`self.K2_GetPawn`)))
  (bind _location (`GameplayStatics.BreakHitResult` (`self.GetHitResultUnderCursorByChannel` "TraceTypeQuery1" false)))
  (`KismetSystemLibrary.DrawDebugArrow` _returnvalue _location 80.0 (make `Object.LinearColor` 0.5))
  (bind _asburglar_c (cast `/Game/Character/Burglar` (`self.K2_GetPawn`)))
  (set `/Game/Character/Burglar.Yaw` (.yaw (`KismetMathLibrary.Conv_VectorToRotator` (- _location _returnvalue))) _asburglar_c))

(fn `UserConstructionScript`)