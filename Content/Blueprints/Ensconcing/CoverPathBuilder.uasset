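; Cover path builder that generates AI cover points along walls between CornersPair corners, run once on first Tick.
; FindStraightCoverPath steps from corner A to B, probing sideways and storing a path unless cover breaks after starting.
; FindSafeHeadAndFeetPosition stacks horizontal traces upward to find safe head height and an agent-radius offset from the nearest hit.
; BuildLevelCoverPaths, uncalled here, only debug-draws unobstructed lines between all corner markers.
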(event EventBeginPlay)

(event EventActorBeginOverlap
  (params (OtherActor :type Actor%20Object%20Reference)))

(event EventTick
  (params (DeltaSeconds :type Float%20%28single-precision%29))
  (Utilities|FlowControl|DoOnce false
    (:Completed
      (bind _outactors (Actor|GetAllActorsOfClass 0 "/Game/Blueprints/Ensconcing/CornersPair.CornersPair_C"))
      (for _array_element _outactors
        (CallFunction|FindStraightCoverPath (Variables|/Game/Blueprints/Ensconcing/CornersPair.CornersPair_C|GetA _array_element) (Variables|/Game/Blueprints/Ensconcing/CornersPair.CornersPair_C|GetB _array_element) 1.5e+02 5e+01 "NewEnumerator1")))))

(fn ConstructionScript)

(fn FindStraightCoverPath
  (params (CornerA :type Corner%20Denotation%20G%20Object%20Reference) (CornerB :type Corner%20Denotation%20G%20Object%20Reference) (AgentHeight :type Float%20%28single-precision%29 :default 0.0) (SearchStep :type Float%20%28single-precision%29 :default 0.0) (SearchDirection :type EWallSide%20Enum :default "NewEnumerator0") (NewPathID_Ignore :type Integer :default 0))
  (bind _returnvalue (Transformation|GetActorLocation CornerA))
  (bind _returnvalue_2 (Transformation|GetActorLocation CornerB))
  (bind _coverpaths (Variables|Default|GetCoverPaths))
  (bind _coverpoints (LocalVariables|GetCoverPoints))
  (bind _returnvalue_3 (Utilities|Array|Length _coverpaths))
  (bind _returnvalue_4 (- _returnvalue_2 _returnvalue))
  (Utilities|FlowControl|Sequence
    (:then_0
      ;[1 1 1] Find path origin, path length, forward, up and right vector of path
      (LocalVariables|SetOriginV _returnvalue)
      (LocalVariables|SetPathLength (Math|Vector|VectorLength _returnvalue_4))
      (bind _output_get (LocalVariables|SetAtoB (Math|Vector|Normalize _returnvalue_4)))
      (bind _output_get_2 (LocalVariables|SetUpV "0, 0,1.000000"))
      (LocalVariables|SetRightV (Math|Vector|Normalize (Math|Vector|CrossProduct _output_get_2 _output_get))))
    (:then_1
      ;[1 1 1] Build cover path
      (while (and (> (LocalVariables|GetPathLength) (LocalVariables|GetCurrentPosition)) (not (LocalVariables|GetNotFound)))
        (switch Utilities|FlowControl|Switch|SwitchonEWallSide SearchDirection
          (:NewEnumerator1
            (bind (_coverpointinfo _notfound _outcoverpointlocation _outmaxsafeheight) (CallFunction|FindSafeHeadandFeetPosition (+ (* (LocalVariables|GetAtoB) (LocalVariables|GetCurrentPosition)) (LocalVariables|GetOriginV)) (* (LocalVariables|GetRightV) -1.0) AgentHeight 1e+01 1e+02 4e+01))
            (if _notfound
              ;;[1 1 1] Break the loop if path is broken
              (if (LocalVariables|GetPathStarted) :!label _label
                (LocalVariables|SetNotFound true) ; Break the loop
                (else
                  ;;[1 1 1] Shift current position along the cover path
                  (LocalVariables|SetCurrentPosition (+ SearchStep (LocalVariables|GetCurrentPosition)) :!label _label_2)))
              (else
                ;;[1 1 1] Collect cover point
                (Utilities|Array|Add _coverpoints (Utilities|Struct|MakeCoverPointInfo _outcoverpointlocation _outmaxsafeheight _returnvalue_3 (LocalVariables|GetCoverPointCount)))
                (LocalVariables|SetCoverPointCount (+ (LocalVariables|GetCoverPointCount) 1) :!label _label_3)
                (LocalVariables|SetPathStarted true)
                (goto _label_2))))
          (:NewEnumerator2
            (bind (_coverpointinfo_2 _notfound_2 _outcoverpointlocation_2 _outmaxsafeheight_2) (CallFunction|FindSafeHeadandFeetPosition (+ (* (LocalVariables|GetAtoB) (LocalVariables|GetCurrentPosition)) (LocalVariables|GetOriginV)) (LocalVariables|GetRightV) 0.0 1e+01 1e+02 4e+01))
            (if _notfound_2
              (goto _label)
              (else
                (Utilities|Array|Add _coverpoints (Utilities|Struct|MakeCoverPointInfo _outcoverpointlocation_2 _outmaxsafeheight_2 _returnvalue_3 (LocalVariables|GetCoverPointCount)))
                (goto _label_3))))))
      (if (LocalVariables|GetNotFound)
        _
        (else
          (CallFunction|AddCoverPath (Utilities|Struct|MakeCoverPath (LocalVariables|GetCoverPoints) SearchDirection))))
      (return (LocalVariables|GetNotFound)))))

(fn BuildLevelCoverPaths
  (bind _outactors (Actor|GetAllActorsOfClass 0 "/Game/Blueprints/Ensconcing/CornerDenotation_G.CornerDenotation_G_C")) ; Get all the corners in the world
  ;[1 1 1] Loop over all possible pairs (O(N^2))
  (for _index (range 0 (- (Utilities|Array|Length _outactors) 2)) ; i=0..N-2
    (for _index_2 (range (+ _index 1) (- (Utilities|Array|Length _outactors) 1)) ; j=(i+1)..N-1
      (bind _returnvalue (Collision|LineTraceByChannel 0 (Transformation|GetActorLocation (Utilities|Array|Get(acopy) _outactors _index_2)) (Transformation|GetActorLocation (Utilities|Array|Get(acopy) _outactors _index)) "TraceTypeQuery1" false 0 "None"))
      (if (not _returnvalue)
        (Rendering|Debug|DrawDebugLine 0 (Transformation|GetActorLocation (Utilities|Array|Get(acopy) _outactors _index_2)) (Transformation|GetActorLocation (Utilities|Array|Get(acopy) _outactors _index)) "(R=1.000000,G=0.000000,B=0.000000,A=1.000000)" 1e+02 1e+01)))))

(fn FindSafeHeadandFeetPosition
  (params (Location :type Vector :default "0, 0, 0") (Direction :type Vector :default "0, 0, 0") (MaxHeight :type Float%20%28single-precision%29 :default 0.0) (Step :type Float%20%28single-precision%29 :default 0.0) (RaycastDistance :type Float%20%28single-precision%29 :default 0.0) (AgentRadius :type Float%20%28single-precision%29 :default 0.0))
  (Utilities|FlowControl|Sequence
    (:then_0
      ;[1 1 1] Define how many rays cast
      (LocalVariables|SetNumRays (Math|Float|Floor (/ MaxHeight Step)))
      (LocalVariables|SetUpV "0, 0,1.000000"))
    (:then_1
      ;[1 1 1] Look for the last ray intersecting point - this is maximum safe height from the ground agent's head can take
      (bind _index (Utilities|FlowControl|ForLoopwithBreak 0 (LocalVariables|GetNumRays) :!label _label)
        (:LoopBody
          (bind (_outhit _returnvalue) (Collision|LineTraceByChannel 0 (+ Location (* (LocalVariables|GetUpV) (* _index Step))) (+ (* Direction RaycastDistance) (+ Location (* (LocalVariables|GetUpV) (* _index Step)))) "TraceTypeQuery1" false 0 "None"))
          ;[1 1 1] Find max safe head height
          (if _returnvalue
            (bind _output_get (LocalVariables|SetLastImpact _outhit))
            (if (< (Math|Vector|VectorLength (- (+ Location (* (LocalVariables|GetUpV) (* _index Step))) (.ImpactPoint (Collision|BreakHitResult _output_get)))) (LocalVariables|GetNearestImpactPoint))
              (LocalVariables|SetNearestImpactPoint (Math|Vector|VectorLength (- (+ Location (* (LocalVariables|GetUpV) (* _index Step))) (.ImpactPoint (Collision|BreakHitResult _output_get))))))
            (else
              (Utilities|FlowControl|Sequence
                (:then_0
                  (goto _label Break))
                (:then_1
                  ;[1 1 1] Get max safe head height
                  (if (== _index 0) :!label _label_2
                    (LocalVariables|SetCoverNotFound true)
                    (return "" (LocalVariables|GetCoverNotFound) (LocalVariables|GetCoverPointLocation) (LocalVariables|GetMaxSafeHeight))
                    (else
                      (LocalVariables|SetMaxSafeHeight (Math|Vector|VectorLength (* (- (.ImpactPoint (Collision|BreakHitResult (LocalVariables|GetLastImpact))) Location) "0.000000,0.000000,1.000000"))))))))))
        (:Completed
          (goto _label_2))))
    (:then_2
      (LocalVariables|SetCoverPointLocation (+ Location (* Direction (- (LocalVariables|GetNearestImpactPoint) AgentRadius))))
      (if (Variables|Default|GetDrawCoverPoints)
        (Rendering|Debug|DrawDebugSphere 0 (+ (+ Location (* Direction (- (LocalVariables|GetNearestImpactPoint) AgentRadius))) (* "0, 0,1.000000" (LocalVariables|GetMaxSafeHeight))) 5.0 8 "(R=0.600000,G=0.004244,B=0.000000,A=1.000000)" 999.0))
      (return "" (LocalVariables|GetCoverNotFound) (LocalVariables|GetCoverPointLocation) (LocalVariables|GetMaxSafeHeight)))))

(fn AddCoverPath
  (params (Path :type Cover%20Path%20Structure%20%28by%20ref%29))
  (Utilities|Array|Add (Variables|Default|GetCoverPaths) Path))