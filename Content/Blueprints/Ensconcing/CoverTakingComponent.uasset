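; Cover component for the Burglar character that finds nearby cover, walks to it and moves along cover paths.
; It searches points from the level's CoverPathBuilder by radius, capsule-trace reachability and distance.
; Tick steers toward the target with straight-line movement input, setting crouch from the point's safe height.
; Axis input steps to neighbouring path points according to wall side, shifting the camera at left-wall path ends.
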(event EventTick
  (params (DeltaSeconds :type Float%20%28single-precision%29))
  (Utilities|FlowControl|Sequence
    (:then_0
      (Utilities|FlowControl|DoOnce false
        (:Completed
          (Utilities|FlowControl|Sequence
            (:then_0
              ;[1 1 1] Find CoverPathBuilder
              (bind _outactors (Actor|GetAllActorsOfClass 0 "/Game/Blueprints/Ensconcing/CoverPathBuilder.CoverPathBuilder_C"))
              (if (> (Utilities|Array|Length _outactors) 0)
                (Variables|Default|SetCoverPathBuilderRef (Utilities|Array|Get(acopy) _outactors))
                (else
                  (Development|PrintText 0 "No CoverPathBuilder found in the World!"))))
            (:then_1
              ;[1 1 1] Get owning Character
              (bind _asburglar (Utilities|Casting|CastToBurglar (Components|GetOwner))
                (:then
                  (Variables|Default|SetMyPawn _asburglar))
                (:CastFailed
                  (Development|PrintString 0 "Owner must be Character!"))))))))
    (:then_1
      ;[1 1 1] Contunue movement to a cover point, if needed
      (if (not (Variables|Default|GetReachedCoverPoint))
        (CallFunction|ContinueMovement (Variables|Default|GetReachTolerance))
        (if (not (Variables|Default|GetWantsCompleteMovement))
          (Variables|Default|SetReachedCoverPoint true))))))

(event EventInitializeComponent)

(fn FindNearestCoverPoint
  (params (Radius :type Float%20%28single-precision%29 :default 0.0) (bDrawDebug :type Boolean :default false))
  (bind _coverpointsinradius (LocalVariables|GetCoverPointsInRadius))
  (bind _mypawn (Variables|Default|GetMyPawn))
  (bind _capsulecomponent (Variables|/Script/Engine.Character|GetCapsuleComponent _mypawn))
  (bind _capsulehalfheight (Variables|/Script/Engine.CapsuleComponent|GetCapsuleHalfHeight _capsulecomponent))
  (if (and (Utilities|IsValid (Variables|Default|GetCoverPathBuilderRef)) (Utilities|IsValid (Variables|Default|GetMyPawn)))
    (LocalVariables|SetDrawDebug bDrawDebug)
    (LocalVariables|SetActorLocation (Transformation|GetActorLocation (Variables|Default|GetMyPawn)))
    (for _array_element (Variables|/Game/Blueprints/Ensconcing/CoverPathBuilder.CoverPathBuilder_C|GetCoverPaths (Variables|Default|GetCoverPathBuilderRef))
      ;[1 1 1] Find cover points in the given radius
      (for _array_element_2 (.CoverPoints (Utilities|Struct|BreakCoverPath _array_element))
        (if (> Radius (Math|Vector|VectorLength (- (Transformation|GetActorLocation (Variables|Default|GetMyPawn)) (.Location (Utilities|Struct|BreakCoverPointInfo _array_element_2)))))
          (Utilities|Array|Add _coverpointsinradius _array_element_2)))
      ;[1 1 1] Check if a cover point could be reached by straight line from the agent
      (for _array_element_3 _coverpointsinradius
        (bind _returnvalue (Class|KismetSystemLibrary|CapsuleTraceSingleNEW 0 (LocalVariables|GetActorLocation) (+ (.Location (Utilities|Struct|BreakCoverPointInfo _array_element_3)) (* "0, 0,1.000000" _capsulehalfheight)) (Variables|/Script/Engine.CapsuleComponent|GetCapsuleRadius _capsulecomponent) _capsulehalfheight "TraceTypeQuery1" false 0 "None" true))
        (if (not _returnvalue)
          (Utilities|Array|Add (LocalVariables|GetVisibleCoverPoints) _array_element_3)))
      ;[1 1 1] Find nearest cover point
      (LocalVariables|SetMinDistance 999999.0)
      (for _array_element_4 (LocalVariables|GetVisibleCoverPoints)
        (if (< (Math|Vector|VectorLength (- (.Location (Utilities|Struct|BreakCoverPointInfo _array_element_4)) (LocalVariables|GetActorLocation))) (LocalVariables|GetMinDistance))
          (LocalVariables|SetMinDistance (Math|Vector|VectorLength (- (.Location (Utilities|Struct|BreakCoverPointInfo _array_element_4)) (LocalVariables|GetActorLocation))))
          (LocalVariables|SetNearestCoverPoint _array_element_4)
          (LocalVariables|SetFound true)))
      (if (and (LocalVariables|GetFound) (LocalVariables|GetDrawDebug))
        (Rendering|Debug|DrawDebugBox 0 (.Location (Utilities|Struct|BreakCoverPointInfo (LocalVariables|GetNearestCoverPoint))) "10.000000,10.000000,10.000000" "(R=0.000000,G=0.227268,B=1.000000,A=1.000000)" "0, 0, 0" 5.0))
      (return (LocalVariables|GetFound) (LocalVariables|GetNearestCoverPoint)))
    (else
      (Development|PrintString 0 "Initialization failure!"))))

(fn MovetoCoverPoint
  (params (CoverPoint :type Cover%20Point%20Info%20Structure) (Tolerance :type Float%20%28single-precision%29 :default 0.0) (CompleteMovement :type Boolean :default false))
  (Variables|Default|SetReachedCoverPoint false)
  (Variables|Default|SetTargetCoverPoint CoverPoint)
  (Variables|Default|SetReachTolerance Tolerance)
  (Variables|Default|SetWantsCompleteMovement CompleteMovement))

(fn ContinueMovement
  (params (ReachTolerance :type Float%20%28single-precision%29 :default 0.0))
  (bind _mypawn (Variables|Default|GetMyPawn))
  (bind _mypawn_2 (Variables|Default|GetMyPawn))
  (if (not (and (Utilities|IsValid (Variables|Default|GetMyPawn)) (Variables|Default|GetReachedCoverPoint)))
    ;[1 1 1] Calc feet location
    (bind _output_get (LocalVariables|SetFeetLocation (- (Transformation|GetActorLocation _mypawn) (* "0, 0,1.000000" (Variables|/Script/Engine.CapsuleComponent|GetCapsuleHalfHeight (Variables|/Script/Engine.Character|GetCapsuleComponent _mypawn))))))
    ;[1 1 1] Reached the goal?
    (bind _output_get_2 (LocalVariables|SetMovementVector (- (.Location (Utilities|Struct|BreakCoverPointInfo (Variables|Default|GetTargetCoverPoint))) _output_get)))
    (if (> (Math|Vector|VectorLength _output_get_2) ReachTolerance)
      ;[1 1 1] Simple move to the goal
      (Pawn|Input|AddMovementInput (Variables|Default|GetMyPawn) (Math|Vector|Normalize (LocalVariables|GetMovementVector)) 1.0 false)
      ;[1 1 1] Crouch if max safe head height is lover than base eye height
      (bind _asburglar (Utilities|Casting|CastToBurglar _mypawn_2))
      (if (> (Variables|/Script/Engine.Pawn|GetBaseEyeHeight _mypawn_2) (* (.MaxSafeHeight (Utilities|Struct|BreakCoverPointInfo (Variables|Default|GetTargetCoverPoint))) 0.5))
        (Default|DoCrouch _asburglar false)
        (else
          (Default|DoCrouch _asburglar true)))
      (else
        (Variables|Default|SetReachedCoverPoint true)
        (Variables|Default|SetIsTakingCover true)
        (Variables|Default|SetCurCoverPoint (Variables|Default|GetTargetCoverPoint))))))

(fn TakeNearestCover
  (params (SearchRadius :type Float%20%28single-precision%29 :default 0.0) (ReachTolerance :type Float%20%28single-precision%29 :default 0.0))
  (bind (_bfound _coverpoint) (CallFunction|FindNearestCoverPoint SearchRadius false))
  (if _bfound
    (CallFunction|MovetoCoverPoint _coverpoint ReachTolerance true)))

(fn StopTakingCover
  (Variables|Default|SetIsTakingCover false)
  (Variables|Default|SetReachedCoverPoint true))

(fn MoveAlongCoverPath
  (params (AxisValue :type Float%20%28single-precision%29 :default 0.0))
  (if (and (Variables|Default|GetIsTakingCover) (!= AxisValue 0.0))
    (bind _coverpoint (CallFunction|FindNextCoverPointinPath (> AxisValue 0.0)))
    (CallFunction|MovetoCoverPoint _coverpoint 2e+01 false)))

(fn FindNextCoverPointinPath
  (params (InRightDirection :type Boolean :default false))
  (bind _curcoverpoint (Variables|Default|GetCurCoverPoint))
  (bind _mypawn (Variables|Default|GetMyPawn))
  (bind _coverpathbuilderref (Variables|Default|GetCoverPathBuilderRef))
  (bind _mypawn_2 (Variables|Default|GetMyPawn))
  (bind (_location _maxsafeheight _pathid _coverpointid) (Utilities|Struct|BreakCoverPointInfo _curcoverpoint))
  (bind _coverpaths (Variables|/Game/Blueprints/Ensconcing/CoverPathBuilder.CoverPathBuilder_C|GetCoverPaths _coverpathbuilderref))
  (bind _item (Utilities|Array|Get(acopy) _coverpaths _pathid))
  (bind (_coverpoints _wallside) (Utilities|Struct|BreakCoverPath _item))
  (if (Variables|Default|GetIsTakingCover)
    (LocalVariables|SetRightDirection InRightDirection)
    (LocalVariables|SetCurCoverPointID _coverpointid)
    (switch Utilities|FlowControl|Switch|SwitchonEWallSide _wallside
      (:NewEnumerator1
        (if (LocalVariables|GetRightDirection) ; LEFT-side wall
          (if (== (- (Utilities|Array|Length _coverpoints) 1) (LocalVariables|GetCurCoverPointID)) ; Wants to move RIGHT (idx increases)
            (Default|ShiftCamera _mypawn_2 1.0)
            (LocalVariables|SetNextCoverPointID (LocalVariables|GetCurCoverPointID) :!label _label) ; Next = Current
            (else
              (Default|ShiftCamera _mypawn_2 0.0)
              (LocalVariables|SetNextCoverPointID (+ (LocalVariables|GetCurCoverPointID) 1) :!label _label_2) ; Next = Idx + 1
            ))
          (elif (== 0 (LocalVariables|GetCurCoverPointID))
            (Default|ShiftCamera _mypawn -1.0)
            (goto _label)
            (else
              (Default|ShiftCamera _mypawn 0.0)
              (LocalVariables|SetNextCoverPointID (- (LocalVariables|GetCurCoverPointID) 1) :!label _label_3)))))
      (:NewEnumerator2
        (if (LocalVariables|GetRightDirection) ; RIGHT-side wall
          (if (== 0 (LocalVariables|GetCurCoverPointID))
            (goto _label)
            (else
              (goto _label_3)))
          (elif (== (- (Utilities|Array|Length _coverpoints) 1) (LocalVariables|GetCurCoverPointID))
            (goto _label)
            (else
              (goto _label_2))))))
    (return (Utilities|Array|Get(acopy) _coverpoints (LocalVariables|GetNextCoverPointID)))))